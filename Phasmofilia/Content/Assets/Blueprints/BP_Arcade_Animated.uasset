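; Animated arcade cabinet that fakes a Flappy Bird-style chicken game on its screen, with one- and two-player variants.
; Timelines drive dynamic material parameters for the title drop, game start, looping chicken flaps and scrolling trees, while Tick alternates wing textures.
; Timeline events switch to tiling trees and trigger optional flap and score sounds.
; Separate events animate button presses and reset the cabinet, toggling desaturation through SetLowProfile.
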(event Custom|Reset
  ;[1 1 1] Reset when restarting
  (CallFunction|SetLowProfile true)
  (CallFunction|ResetArcade)
  (Utilities|FlowControl|Sequence
    (:then_0
      ;[1 1 1] Show gameplay
      (Utilities|FlowControl|DoOnce false) ; enters at Reset
    )
    (:then_1
      (Utilities|FlowControl|Gate true) ; enters at Close
    )))

(event Custom|Start%20game
  (bind _returnvalue (Transformation|GetActorLocation))
  (bind _arcade_screen (Variables|Default|GetArcade%20screen))
  (bind _arcade_screen_2 (Variables|Default|GetArcade%20screen))
  (bind _arcade_screen_3 (Variables|Default|GetArcade%20screen))
  (bind _returnvalue_2 (+ _returnvalue "0, 0,180.000000"))
  ;[1 1 1] Show gameplay
  (Audio|Components|Audio|Stop (Variables|Default|GetTitle%20drop))
  (bind (_direction _drop _move_back) (Timeline|Gameplay%20start PlayFromStart)
    (:Update
      (Rendering|Material|SetScalarParameterValue _arcade_screen "Title position" _drop :!class /Script/Engine.MaterialInstanceDynamic) ; Raise title screen
      (Rendering|Material|SetVectorParameterValue _arcade_screen "Position" (Math|Conversions|ToLinearColor(Vector) (Math|Vector|MakeVector _move_back 0.35 0.0)) :!class /Script/Engine.MaterialInstanceDynamic) ; Move chicken 1
      (Rendering|Material|SetVectorParameterValue _arcade_screen "Position2" (Math|Conversions|ToLinearColor(Vector) (Math|Vector|MakeVector _move_back (Math|Float|Lerp 0.55 0.35 _drop) 0.0)) :!class /Script/Engine.MaterialInstanceDynamic) ; Move chicken 2
    )
    (:Finished
      (Utilities|FlowControl|Sequence
        (:then_0
          (bind (_direction_2 _height _rotation _height2 _rotation2) (Timeline|Tapping%20loop PlayFromStart) ; Looping flappy animation
            (:Update
              (Rendering|Material|SetVectorParameterValue _arcade_screen_2 "Position" (Math|Conversions|ToLinearColor(Vector) (Math|Vector|MakeVector 0.15 _height _rotation)) :!class /Script/Engine.MaterialInstanceDynamic) ; Flap chicken 1
              (Rendering|Material|SetVectorParameterValue _arcade_screen_2 "Position2" (Math|Conversions|ToLinearColor(Vector) (Math|Vector|MakeVector 0.15 _height2 _rotation2)) :!class /Script/Engine.MaterialInstanceDynamic) ; Flap chicken 2
            )
            (:Flap
              (Utilities|FlowControl|FlipFlop
                (:A
                  (if (Variables|Default|GetPlay%20sounds) :!label _label
                    (Audio|PlaySoundatLocation "/Game/Assets/Audio/Arcade/SFX_FlapWing_Cue.SFX_FlapWing_Cue" _returnvalue_2 "0, 0, 0" 1.0 1.0 0.0 0 0 0) ; Flapping sound
                  ))
                (:B
                  (if (Variables|Default|Get2%20Player)
                    (goto _label)))))))
        (:then_1
          (bind _tree_movement (Timeline|Tree%20loop PlayFromStart)
            (:Update
              (Rendering|Material|SetScalarParameterValue _arcade_screen_3 "Tree position" _tree_movement :!class /Script/Engine.MaterialInstanceDynamic) ; Move trees left
            )
            (:Tree%20looping
              (Utilities|FlowControl|DoOnce false
                (:Completed
                  (Rendering|Material|SetTextureParameterValue _arcade_screen_3 "Trees" "/Game/Assets/Textures/T_Arcade_Trees_Tiling.T_Arcade_Trees_Tiling") ; Switch to tiling tree texture
                  (Utilities|FlowControl|Sequence
                    (:then_0
                      (goto _label_3 Open))
                    (:then_1
                      (if (Variables|Default|GetPlay%20sounds) :!label _label_2
                        (Audio|PlaySoundatLocation "/Game/Assets/Audio/Arcade/SFX_Score_01_Cue.SFX_Score_01_Cue" _returnvalue_2 "0, 0, 0" 1.0 1.0 0.0 0 0 0) ; Score sound
                      ))))))
            (:Score
              (Utilities|FlowControl|Gate true :!label _label_3
                (:Exit
                  (goto _label_2))))))))))

(event Custom|Left%20button%20press
  ;[1 1 1] Button press anims
  (bind _press (Timeline|Left%20press PlayFromStart)
    (:Update
      (Transformation|SetRelativeLocation (Variables|Default|GetLeft%20button) (Math|Vector|MakeVector 0.0 26.8 _press) false false))))

(event Custom|Right%20button%20press
  ;[1 1 1] Button press anims
  (bind _press (Timeline|Right%20press PlayFromStart)
    (:Update
      (Transformation|SetRelativeLocation (Variables|Default|GetRight%20button) (Math|Vector|MakeVector 0.0 -26.8 _press) false false))))

(event Custom|Show%20title
  (bind _arcade_screen (Variables|Default|GetArcade%20screen))
  ;[1 1 1] Show title screen
  (CallFunction|SetLowProfile false)
  (CallFunction|ResetArcade)
  (bind (_direction _drop _position2 _position) (Timeline|Title%20drop PlayFromStart)
    (:Update
      (Rendering|Material|SetScalarParameterValue _arcade_screen "Title position" _drop :!class /Script/Engine.MaterialInstanceDynamic)
      (Rendering|Material|SetVectorParameterValue _arcade_screen "Position" (Math|Color|MakeColor (.X (Math|Vector|BreakVector _position)) (.Y (Math|Vector|BreakVector _position)) 0.0) :!class /Script/Engine.MaterialInstanceDynamic)
      (Rendering|Material|SetVectorParameterValue _arcade_screen "Position2" (Math|Color|MakeColor (.X (Math|Vector|BreakVector _position)) _position2 0.0) :!class /Script/Engine.MaterialInstanceDynamic)
      (Rendering|Material|SetScalarParameterValue _arcade_screen "Tree position" 0.0 :!class /Script/Engine.MaterialInstanceDynamic))))

(event EventInteract
  (CallFunction|StartGame))

(event EventTick
  (params (DeltaSeconds :type Float%20%28single-precision%29))
  (bind _arcade_screen (Variables|Default|GetArcade%20screen))
  ;[1 1 1] Chicken flap textures
  (Utilities|FlowControl|Delay 0.12)
  (Utilities|FlowControl|FlipFlop
    (:A
      (Rendering|Material|SetTextureParameterValue _arcade_screen "Chicken" "/Game/Assets/Textures/T_Arcade_Chicken.T_Arcade_Chicken")
      (Rendering|Material|SetTextureParameterValue _arcade_screen "Chicken2" "/Game/Assets/Textures/T_Arcade_Chicken_3.T_Arcade_Chicken_3"))
    (:B
      (Rendering|Material|SetTextureParameterValue _arcade_screen "Chicken" "/Game/Assets/Textures/T_Arcade_Chicken_2.T_Arcade_Chicken_2")
      (Rendering|Material|SetTextureParameterValue _arcade_screen "Chicken2" "/Game/Assets/Textures/T_Arcade_Chicken_4.T_Arcade_Chicken_4"))))

(event EventBeginPlay
  ;[1 1 1] Show gameplay
  (Utilities|FlowControl|Delay 1.0))

(fn ConstructionScript
  (if (Variables|Default|Get2%20Player)
    _
    (else
      (Rendering|Material|SetMaterial (Variables|Default|GetArcade) 1 "/Game/Assets/Materials/M_Arcade_Screen_1player.M_Arcade_Screen_1player")))
  (bind _returnvalue (Rendering|Material|CreateDynamicMaterialInstance (Variables|Default|GetArcade) 0 0 "None" :!class /Script/Engine.PrimitiveComponent))
  (Variables|Default|SetCabinet%20material _returnvalue)
  (Rendering|Material|SetMaterial (Variables|Default|GetRight%20button) 0 (Variables|Default|GetCabinet%20material))
  (bind _returnvalue_2 (Rendering|Material|CreateDynamicMaterialInstance (Variables|Default|GetArcade) 1 0 "None" :!class /Script/Engine.PrimitiveComponent))
  (Variables|Default|SetArcade%20screen _returnvalue_2)
  (CallFunction|SetLowProfile (Variables|Default|GetLow%20profile)))

(fn SetLowProfile
  (params (Low%20profile :type Boolean))
  (Rendering|Material|SetScalarParameterValue (Variables|Default|GetCabinet%20material) "Desaturation" (Math|Float|SelectFloat 1.0 0.0 Low%20profile) :!class /Script/Engine.MaterialInstanceDynamic)
  (return))

(fn ResetArcade
  (bind _arcade_screen (Variables|Default|GetArcade%20screen))
  (Audio|Components|Audio|Stop (Variables|Default|GetTitle%20drop))
  (Rendering|Material|SetScalarParameterValue _arcade_screen "Title position" 1.0 :!class /Script/Engine.MaterialInstanceDynamic)
  (Rendering|Material|SetScalarParameterValue _arcade_screen "Tree position" 0.0 :!class /Script/Engine.MaterialInstanceDynamic)
  (Rendering|Material|SetVectorParameterValue _arcade_screen "Position" "(R=0.500000,G=0.350000,B=0.000000,A=1.000000)" :!class /Script/Engine.MaterialInstanceDynamic)
  (Rendering|Material|SetTextureParameterValue _arcade_screen "Trees" "/Game/Assets/Textures/T_Arcade_Trees.T_Arcade_Trees")
  (Variables|Default|SetPlay%20sounds false))