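; BP_DoorwayJumpscare is a jumpscare actor that slides a mannequin to an endpoint, by its name across a doorway.
; While CalledJumpscare is true, Tick moves Mannequin toward Endpoint's world location with VInterpToConstant at a constant Speed, without sweeping.
; The actor destroys itself once the mannequin arrives.
; Nothing in this graph sets CalledJumpscare, so the scare relies on an outside trigger.
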(event EventBeginPlay)

(event Collision|EventActorBeginOverlap
  (params (OtherActor :type Actor%20Object%20Reference)))

(event EventTick
  (params (DeltaSeconds :type Float%20%28single-precision%29))
  (if (Variables|Default|GetcalledJumpscare)
    (Transformation|SetWorldLocation (Variables|Default|GetMannequin) (Math|Interpolation|VInterptoConstant (Transformation|GetWorldLocation (Variables|Default|GetMannequin)) (Transformation|GetWorldLocation (Variables|Default|GetEndpoint)) DeltaSeconds (Variables|Default|GetSpeed)) false false)
    (if (Math|Vector|Equal(Vector) (Transformation|GetWorldLocation (Variables|Default|GetMannequin)) (Transformation|GetWorldLocation (Variables|Default|GetEndpoint)) 0.0001)
      (Actor|DestroyActor))))

(fn ConstructionScript)