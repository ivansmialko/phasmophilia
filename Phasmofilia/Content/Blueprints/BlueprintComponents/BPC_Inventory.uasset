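; Inventory component that stores item stacks in player-controller-sized slots and handles adding, using, removing, dropping and slot expansion.
; AddItem fills partial stacks, then empty slots, recursing on overflow and reporting any remainder, while each change refreshes the matching grid widget.
; UseItem calls UseItem on an existing or newly spawned item actor; DropItem spawns a physics pickup via camera trace.
; It also creates and opens the examination widget.
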(event Custom|Initialize)

(event Custom|CreateExaminationWidget
  (params (Index :type Integer))
  (bind _inventory_menu_instance (Variables|Default|GetInventory%20Menu%20Instance))
  (Default|UpdateWidget (Variables|Default|GetExaminationWidgetInstance) Index)
  (Widget|SetVisibility (Variables|Default|GetInventory%20Menu%20Instance) "Collapsed")
  (Utilities|IsValid (Variables|/Game/UMG/Inventory/W_IntentoryMenu.W_IntentoryMenu_C|GetW_InventoryDropdown _inventory_menu_instance)
    (:Is%20Valid
      (Default|CloseDropdownMenu _inventory_menu_instance))
    (:Is%20Not%20Valid
      _))
  (UserInterface|Viewport|AddtoViewport (Variables|Default|GetExaminationWidgetInstance) 2)
  (Variables|/Game/GameBP/HG_PlayerController.HG_PlayerController_C|SetisInventoryOpen (.AsHG%20Player%20Controller (Utilities|Casting|CastToHG_PlayerController (Game|GetPlayerController 0))) false))

(event EventBeginPlay
  (bind _returnvalue (Game|GetPlayerController 0))
  (bind _ashg_player_controller (Utilities|Casting|CastToHG_PlayerController _returnvalue))
  (Utilities|Array|Resize (Variables|Default|GetInventorySlots) (Variables|/Game/GameBP/HG_PlayerController.HG_PlayerController_C|GetInventorySlotsAmount _ashg_player_controller))
  (Variables|Default|SetInventory%20Menu%20Instance (Variables|/Game/GameBP/HG_PlayerController.HG_PlayerController_C|GetInventoryMenuInstance _ashg_player_controller))
  (bind _asl1_character (Utilities|Casting|CastToL1_Character (Game|GetPlayerCharacter 0)))
  (Variables|Default|SetPlayerCharacterInstance _asl1_character)
  (bind _returnvalue_2 (UserInterface|CreateWidget "/Game/UMG/Inventory/W_Examination.W_Examination_C" 0 0))
  (Variables|Default|SetExaminationWidgetInstance _returnvalue_2)
  (bind _outactors (Actor|GetAllActorsOfClass "/Game/Blueprints/Actors/Inventory/BP_Examination.BP_Examination_C"))
  (Variables|Default|SetBP_ExaminationInstance (Utilities|Array|Get(acopy) _outactors))
  (Variables|/Game/UMG/Inventory/W_Examination.W_Examination_C|SetBPC_InventoryInstance (Variables|Default|GetExaminationWidgetInstance) self)
  (Variables|/Game/GameBP/HG_PlayerController.HG_PlayerController_C|SetW_ExaminationWidgetInstance (.AsHG%20Player%20Controller (Utilities|Casting|CastToHG_PlayerController (Game|GetPlayerController 0))) (Variables|Default|GetExaminationWidgetInstance)))

(fn AddItem
  (params (Item :type BP%20Inventory%20Item%20Base%20Class%20Reference) (Amount :type Integer))
  (bind (_success_ _index) (CallFunction|CheckforEmptySlot))
  (bind (_success__2 _index_2) (CallFunction|CheckforEmptySlot))
  (LocalVariables|SetLocalItem Item)
  (LocalVariables|SetLocalAmount Amount)
  (LocalVariables|SetLocalMaxStackAmount (.MaxStackAmount (Utilities|Struct|BreakS_ItemData (Utilities|GetClassDefaults (LocalVariables|GetLocalItem)))))
  (if (> (.MaxStackAmount (Utilities|Struct|BreakS_ItemData (Utilities|GetClassDefaults (LocalVariables|GetLocalItem)))) 1)
    (bind (_success__3 _index_3) (CallFunction|CheckforAvailableSlot (LocalVariables|GetLocalItem)))
    (if _success__3
      (LocalVariables|SetLocalIndex _index_3)
      (if (> (+ (.Amount (CallFunction|GetItemDataatIndex (LocalVariables|GetLocalIndex))) (LocalVariables|GetLocalAmount)) (LocalVariables|GetLocalMaxStackAmount))
        (LocalVariables|SetLocalAmount (- (+ (.Amount (CallFunction|GetItemDataatIndex (LocalVariables|GetLocalIndex))) (LocalVariables|GetLocalAmount)) (LocalVariables|GetLocalMaxStackAmount)))
        (Utilities|Array|SetArrayElem (Variables|Default|GetInventorySlots) (LocalVariables|GetLocalIndex) (Utilities|Struct|MakeS_InventoryStack (LocalVariables|GetLocalItem) (LocalVariables|GetLocalMaxStackAmount)))
        (CallFunction|UpdateInventorySlot (LocalVariables|GetLocalIndex))
        (bind _remainder (CallFunction|AddItem (LocalVariables|GetLocalItem) (LocalVariables|GetLocalAmount)))
        (return true _remainder)
        (else
          (Utilities|Array|SetArrayElem (Variables|Default|GetInventorySlots) (LocalVariables|GetLocalIndex) (Utilities|Struct|MakeS_InventoryStack (LocalVariables|GetLocalItem) (+ (.Amount (CallFunction|GetItemDataatIndex (LocalVariables|GetLocalIndex))) (LocalVariables|GetLocalAmount))))
          (CallFunction|UpdateInventorySlot (LocalVariables|GetLocalIndex))
          (return true 0)))
      (elif _success_
        (LocalVariables|SetLocalIndex _index)
        (if (> (LocalVariables|GetLocalAmount) (LocalVariables|GetLocalMaxStackAmount))
          (Utilities|Array|SetArrayElem (Variables|Default|GetInventorySlots) (LocalVariables|GetLocalIndex) (Utilities|Struct|MakeS_InventoryStack (LocalVariables|GetLocalItem) (LocalVariables|GetLocalMaxStackAmount)))
          (CallFunction|UpdateInventorySlot (LocalVariables|GetLocalIndex))
          (bind (_success__4 _remainder_2) (CallFunction|AddItem (LocalVariables|GetLocalItem) (- (LocalVariables|GetLocalAmount) (LocalVariables|GetLocalMaxStackAmount))))
          (return _success__4 _remainder_2)
          (else
            (Utilities|Array|SetArrayElem (Variables|Default|GetInventorySlots) (LocalVariables|GetLocalIndex) (Utilities|Struct|MakeS_InventoryStack (LocalVariables|GetLocalItem) (LocalVariables|GetLocalAmount)))
            (CallFunction|UpdateInventorySlot (LocalVariables|GetLocalIndex))
            (CallFunction|PlaySoundPickUp)
            (return true 0)))
        (else
          (return false (LocalVariables|GetLocalAmount)))))
    (elif _success__2
      (LocalVariables|SetLocalIndex _index_2)
      (Utilities|Array|SetArrayElem (Variables|Default|GetInventorySlots) (LocalVariables|GetLocalIndex) (Utilities|Struct|MakeS_InventoryStack (LocalVariables|GetLocalItem) 1))
      (CallFunction|UpdateInventorySlot (LocalVariables|GetLocalIndex))
      (if (> (- (LocalVariables|GetLocalAmount) 1) 0)
        (bind _remainder_3 (CallFunction|AddItem (LocalVariables|GetLocalItem) (- (LocalVariables|GetLocalAmount) 1)))
        (return true _remainder_3)
        (else
          (return true 0)))
      (else
        (Development|PrintString "No free slots")
        (return false (LocalVariables|GetLocalAmount))))))

(fn CheckforEmptySlot
  (bind (_array_element _array_index) (Utilities|Array|ForEachLoopwithBreak (Variables|Default|GetInventorySlots) :!label _label)
    (:LoopBody
      (if (Utilities|IsValidClass (.Item (Utilities|Struct|BreakS_InventoryStack _array_element)))
        (LocalVariables|SetlocalSuccess false)
        (else
          (LocalVariables|SetlocalSuccess true)
          (LocalVariables|SetlocalIndex _array_index)
          (goto _label Break))))
    (:Completed
      (return (LocalVariables|GetlocalSuccess) (LocalVariables|GetlocalIndex)))))

(fn GetItemDataatIndex
  (params (Index :type Integer))
  (bind _inventoryslots (Variables|Default|GetInventorySlots))
  (bind _output (Utilities|Array|Get(acopy) _inventoryslots Index))
  (bind (_item _amount) (Utilities|Struct|BreakS_InventoryStack _output))
  (return _item _amount))

(fn UpdateInventorySlot
  (params (Index :type Integer))
  (Default|UpdateSlot (Utilities|Array|Get(acopy) (Variables|/Game/UMG/Inventory/W_InventoryGrid.W_InventoryGrid_C|GetSlotsArray (Variables|/Game/UMG/Inventory/W_IntentoryMenu.W_IntentoryMenu_C|GetW_InventoryGrid (Variables|/Game/GameBP/HG_PlayerController.HG_PlayerController_C|GetInventoryMenuInstance (.AsHG%20Player%20Controller (Utilities|Casting|CastToHG_PlayerController (Game|GetPlayerController 0)))))) Index)))

(fn CheckforAvailableSlot
  (params (NewParam :type BP%20Inventory%20Item%20Base%20Class%20Reference))
  (bind (_array_element _array_index) (Utilities|Array|ForEachLoopwithBreak (Variables|Default|GetInventorySlots) :!label _label)
    (:LoopBody
      (if (and (== (.Item (Utilities|Struct|BreakS_InventoryStack _array_element)) NewParam) (< (.Amount (Utilities|Struct|BreakS_InventoryStack _array_element)) (.maxstackamount (Utilities|GetClassDefaults NewParam))))
        (LocalVariables|SetLocalSuccess true)
        (LocalVariables|SetLocalIndex _array_index)
        (goto _label Break)
        (else
          (LocalVariables|SetLocalSuccess false))))
    (:Completed
      (return (LocalVariables|GetLocalSuccess) (LocalVariables|GetLocalIndex)))))

(fn UseItem
  (params (Index :type Integer))
  (bind _output_get (LocalVariables|SetLocalIndex Index))
  (LocalVariables|SetLocalItem (.Item (CallFunction|GetItemDataatIndex _output_get)))
  (LocalVariables|SetLocalAmount (.Amount (CallFunction|GetItemDataatIndex _output_get)))
  (if (> (LocalVariables|GetLocalAmount) 0)
    (bind _returnvalue (Actor|GetActorOfClass (LocalVariables|GetLocalItem)))
    (Utilities|IsValid _returnvalue
      (:Is%20Valid
        (Default|UseItem _returnvalue))
      (:Is%20Not%20Valid
        (bind _returnvalue_2 (Game|SpawnActorfromClass (LocalVariables|GetLocalItem) (Math|Transform|MakeTransform "0, 0, 0" "0, 0, 0" "1,1,1") "Undefined" 0 0))
        (Default|UseItem _returnvalue_2)))
    (CallFunction|RemoveItem (LocalVariables|GetLocalIndex))
    (Default|CloseDropdownMenu (Variables|Default|GetInventory%20Menu%20Instance))))

(fn RemoveItem
  (params (Index :type Integer))
  (bind _output_get (LocalVariables|SetLocalIndex Index))
  (LocalVariables|SetLocalItem (.Item (CallFunction|GetItemDataatIndex _output_get)))
  (LocalVariables|SetLocalAmount (.Amount (CallFunction|GetItemDataatIndex _output_get)))
  (if (> (LocalVariables|GetLocalAmount) 1)
    (Utilities|Array|SetArrayElem (Variables|Default|GetInventorySlots) (LocalVariables|GetLocalIndex) (Utilities|Struct|MakeS_InventoryStack (LocalVariables|GetLocalItem) (- (LocalVariables|GetLocalAmount) 1)))
    (else
      (Utilities|Array|SetArrayElem (Variables|Default|GetInventorySlots) (LocalVariables|GetLocalIndex) (Utilities|Struct|MakeS_InventoryStack 0 0))))
  (CallFunction|UpdateInventorySlot (LocalVariables|GetLocalIndex)))

(fn DropItem
  (params (Index :type Integer))
  (bind _playercharacterinstance (Variables|Default|GetPlayerCharacterInstance))
  (bind _camera (Variables|/Game/GameBP/Level1/L1_Character.L1_Character_C|GetCamera _playercharacterinstance))
  (bind _returnvalue (Transformation|GetWorldLocation _camera))
  (LocalVariables|SetLocalIndex Index)
  (LocalVariables|SetLocalPickupActorClass (.Item (CallFunction|GetItemDataatIndex (LocalVariables|GetLocalIndex))))
  (LocalVariables|SetLocalAmount (.Amount (CallFunction|GetItemDataatIndex (LocalVariables|GetLocalIndex))))
  (if (> (LocalVariables|GetLocalAmount) 0)
    (for _index (range 0 (- (LocalVariables|GetLocalAmount) 1))
      (CallFunction|RemoveItem (LocalVariables|GetLocalIndex)))
    (Default|CloseDropdownMenu (Variables|Default|GetInventory%20Menu%20Instance))
    (bind (_outhit _returnvalue_2) (Collision|LineTraceByChannel _returnvalue (+ _returnvalue (* (Math|Vector|GetForwardVector _camera) 2e+02)) "TraceTypeQuery1" false 0 "None"))
    (bind _returnvalue_3 (Game|SpawnActorfromClass (.pickupactor (Utilities|GetClassDefaults (LocalVariables|GetLocalPickupActorClass))) (Math|Transform|MakeTransform (select _returnvalue_2 (.location _outhit) (.traceend _outhit)) "0, 0, 0" "1,1,1") "Undefined" 0 0))
    (bind _output_get (Variables|/Game/Blueprints/Actors/Inventory/PickupActors/BP_PickupActorBase.BP_PickupActorBase_C|SetAmount _returnvalue_3 (LocalVariables|GetLocalAmount)))
    (Development|PrintString (Utilities|String|ToString(Integer) _output_get))
    (Physics|SetSimulatePhysics (Variables|/Game/Blueprints/Actors/Inventory/PickupActors/BP_PickupActorBase.BP_PickupActorBase_C|GetStaticMesh _returnvalue_3) true)))

(fn PlaySoundPickUp
  (Default|PlayItemPickUp (Variables|/Game/GameBP/HG_PlayerController.HG_PlayerController_C|GetAudioManagerInstance (.AsHG%20Player%20Controller (Utilities|Casting|CastToHG_PlayerController (Game|GetPlayerController 0))))))

(fn AddMoreSlots
  (params (Amount :type Integer))
  (bind _returnvalue (Game|GetPlayerController 0))
  (bind _inventory_menu_instance (Variables|Default|GetInventory%20Menu%20Instance))
  (bind _ashg_player_controller (Utilities|Casting|CastToHG_PlayerController _returnvalue))
  (bind _w_inventorygrid (Variables|/Game/UMG/Inventory/W_IntentoryMenu.W_IntentoryMenu_C|GetW_InventoryGrid _inventory_menu_instance))
  (bind _output_get (Variables|/Game/GameBP/HG_PlayerController.HG_PlayerController_C|SetInventorySlotsAmount _ashg_player_controller (+ Amount (Variables|/Game/GameBP/HG_PlayerController.HG_PlayerController_C|GetInventorySlotsAmount _ashg_player_controller))))
  (Utilities|Array|Resize (Variables|Default|GetInventorySlots) _output_get)
  (Default|AddMoreSlots _w_inventorygrid Amount)
  (for _array_element (Variables|/Game/UMG/Inventory/W_InventoryGrid.W_InventoryGrid_C|GetSlotsArray _w_inventorygrid)
    (Default|Initialize _array_element (Variables|Default|GetInventory%20Menu%20Instance))))