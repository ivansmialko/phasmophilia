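; Movement component that adds stamina-limited sprinting to a character passed in through Initialize.
; StartSprint switches to sprint speed when stamina and velocity allow, and a looping timer drains stamina while moving, stopping the sprint at minimum.
; StopSprint restores walk speed and, after a retriggerable delay, starts a regeneration timer that refills stamina to maximum.
; Stamina values are printed on screen as they change.
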(event Custom|StartSprint
  (Utilities|Time|ClearTimerbyFunctionName 0 "RegenerateStamina")
  (if (and (> (Variables|Default|GetCurrentStamina) (Variables|Default|GetMinStamina)) (> (Math|Vector|VectorLength (Transformation|GetVelocity (Variables|Default|GetPlayerRef))) 1e+01))
    (CallFunction|SetPlayerMaxWalkSpeed (Variables|Default|GetSprintSpeed))
    (Utilities|Time|SetTimerbyFunctionName 0 "SprintTimerTick" 0.1 true)))

(event Custom|SprintTimerTick
  (if (> (Math|Vector|VectorLength (Transformation|GetVelocity (Variables|Default|GetPlayerRef))) 1e+01)
    (bind _output_get (Variables|Default|SetCurrentStamina (Math|Float|Clamp(Float) (- (Variables|Default|GetCurrentStamina) 1.0) (Variables|Default|GetMinStamina) (Variables|Default|GetMaxStamina))))
    (Development|PrintString (Utilities|String|ToString(Float) _output_get))
    (if (<= (Variables|Default|GetCurrentStamina) (Variables|Default|GetMinStamina))
      (CallFunction|StopSprint))))

(event Custom|StopSprint
  (Utilities|Time|ClearTimerbyFunctionName 0 "SprintTImerTick")
  (CallFunction|SetPlayerMaxWalkSpeed (Variables|Default|GetWalkSpeed))
  (Utilities|FlowControl|RetriggerableDelay 5.0)
  (if (not (Class|KismetSystemLibrary|IsTimerActive 0 "SprintTimerTick"))
    (Utilities|Time|SetTimerbyFunctionName 0 "RegenerateStamina" 0.3 true)))

(event Custom|RegenerateStamina
  (Variables|Default|SetCurrentStamina (Math|Float|Clamp(Float) (+ (Variables|Default|GetCurrentStamina) 1.0) (Variables|Default|GetMinStamina) (Variables|Default|GetMaxStamina)))
  (Development|PrintString (Utilities|String|ToString(Float) (Variables|Default|GetCurrentStamina)))
  (if (>= (Variables|Default|GetCurrentStamina) (Variables|Default|GetMaxStamina))
    (Utilities|Time|ClearTimerbyFunctionName 0 "RegenerateStamina")))

(fn Initialize
  (params (Character :type Character%20Object%20Reference))
  (Variables|Default|SetPlayerRef Character)
  (Variables|/Script/Engine.CharacterMovementComponent|SetMaxWalkSpeed (Variables|/Script/Engine.Character|GetCharacterMovement (Variables|Default|GetPlayerRef)) (Variables|Default|GetWalkSpeed)))

(fn SetPlayerMaxWalkSpeed
  (params (Max%20Walk%20Speed :type Float%20%28single-precision%29))
  (Variables|/Script/Engine.CharacterMovementComponent|SetMaxWalkSpeed (Variables|/Script/Engine.Character|GetCharacterMovement (Variables|Default|GetPlayerRef)) Max%20Walk%20Speed))