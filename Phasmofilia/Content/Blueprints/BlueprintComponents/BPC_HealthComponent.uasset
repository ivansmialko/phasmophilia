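; Health component that tracks current health and drives a blood screen effect from it.
; RemoveHealth and AddHealth clamp the value between the minimum and maximum, then refresh the effect, which also updates on BeginPlay.
; UpdateBloodScreen maps health, from minimum up to 70% of the max-min span, onto the Amount scalar of the global MPC_BloodScreen material parameter collection.
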(event EventBeginPlay
  (CallFunction|UpdateBloodScreen))

(event EventTick
  (params (DeltaSeconds :type Float%20%28single-precision%29)))

(fn RemoveHealth
  (params (Amount :type Float%20%28single-precision%29))
  (Variables|Default|SetCurrentHealth (Math|Float|Clamp(Float) (- (Variables|Default|GetCurrentHealth) Amount) (Variables|Default|GetMinHealth) (Variables|Default|GetMaxHealth)))
  (CallFunction|UpdateBloodScreen))

(fn AddHealth
  (params (Amount :type Float%20%28single-precision%29))
  (Variables|Default|SetCurrentHealth (Math|Float|Clamp(Float) (+ Amount (Variables|Default|GetCurrentHealth)) (Variables|Default|GetMinHealth) (Variables|Default|GetMaxHealth)))
  (CallFunction|UpdateBloodScreen))

(fn UpdateBloodScreen
  (Rendering|Material|SetScalarParameterValue "/Game/Materials/MPC_BloodScreen.MPC_BloodScreen" "Amount" (Math|Float|MapRangeClamped (Variables|Default|GetCurrentHealth) (Variables|Default|GetMinHealth) (* (- (Variables|Default|GetMaxHealth) (Variables|Default|GetMinHealth)) 0.7) 0.5 1.0) :!class /Script/Engine.KismetMaterialLibrary))