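; BP_AudioManager is a central sound manager exposing one event per game sound effect, covering item pickup, flashlight, doors, lockers, levers and brick wall building.
; Pickup and flashlight events play non-spatialized 2D sounds.
; World events take a source actor and play their sound at that actor's location as fire-and-forget one-shots.
; The PlayAmbient event is an empty stub.
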(event Custom|PlayAmbient)

(event Custom|PlayDoorClose
  (params (LocationActor :type Actor%20Object%20Reference))
  (Audio|PlaySoundatLocation "/Game/Sounds/door_close.door_close" (Transformation|GetActorLocation LocationActor) "0, 0, 0" 1.0 1.0 0.0 0 0 0))

(event Custom|PlayMetalLeverSwitch
  (params (Sound%20Source%20Actor :type Actor%20Object%20Reference))
  (Audio|PlaySoundatLocation "/Game/Sounds/metal_lever_switch.metal_lever_switch" (Transformation|GetActorLocation Sound%20Source%20Actor) "0, 0, 0" 1.0 1.0 0.0 0 0 0))

(event Custom|PlayBrickWallBuilding
  (params (Sound%20Source%20Actor :type Actor%20Object%20Reference))
  (Audio|PlaySoundatLocation "/Game/Sounds/wall_bricks_build.wall_bricks_build" (Transformation|GetActorLocation Sound%20Source%20Actor) "0, 0, 0" 1.0 1.0 0.0 0 0 0))

(event Custom|PlayDoorOpen
  (params (LocationActor :type Actor%20Object%20Reference))
  (Audio|PlaySoundatLocation "/Game/Sounds/door_open.door_open" (Transformation|GetActorLocation LocationActor) "0, 0, 0" 1.0 1.0 0.0 0 0 0))

(event Custom|PlayLockerDoorClose
  (params (LocationActor :type Actor%20Object%20Reference))
  (Audio|PlaySoundatLocation "/Game/Sounds/locker_close_door.locker_close_door" (Transformation|GetActorLocation LocationActor) "0, 0, 0" 1.0 1.0 0.0 0 0 0))

(event Custom|PlayItemPickUp
  (Audio|PlaySound2D "/Game/Sounds/item_pick_up.item_pick_up" 1.0 1.0 0.0 0 0))

(event Custom|PlayLockerDoorOpen
  (params (LocationActor :type Actor%20Object%20Reference))
  (Audio|PlaySoundatLocation "/Game/Sounds/locker_open_door.locker_open_door" (Transformation|GetActorLocation LocationActor) "0, 0, 0" 1.0 1.0 0.0 0 0 0))

(event Custom|PlayMetalHeavyDoorMoving
  (params (SoundSourceActor :type Actor%20Object%20Reference))
  (Audio|PlaySoundatLocation "/Game/Sounds/MetalHeavyDoor/metal_heavy_door_move.metal_heavy_door_move" (Transformation|GetActorLocation SoundSourceActor) "0, 0, 0" 1.0 1.0 0.0 0 0 0))

(event Custom|PlayFlashlightOff
  (Audio|PlaySound2D "/Game/Sounds/flashlight_off.flashlight_off" 1.0 1.0 0.0 0 0))

(event Custom|PlayFlashlightOn
  (Audio|PlaySound2D "/Game/Sounds/flashlight_on.flashlight_on" 1.0 1.0 0.0 0 0))

(event Custom|PlayMetalHeavyDoorFinished
  (params (SoundSourceActor :type Actor%20Object%20Reference))
  (Audio|PlaySoundatLocation "/Game/Sounds/MetalHeavyDoor/metal_heavy_door_finished.metal_heavy_door_finished" (Transformation|GetActorLocation SoundSourceActor) "0, 0, 0" 1.0 1.0 0.0 0 0 0))

(fn ConstructionScript)