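; A trigger box actor that switches the player's view to a referenced fixed camera, ReferenceRECamera, when an L1_Character enters it.
; On overlap it blends the view target over briefly, aligns control rotation to the camera's yaw, disables the character's head bob and ignores look input.
; The construction script sizes the box from its BoxExtent variable.
; Nothing in this actor restores the view or look input on exit.
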(event OnComponentBeginOverlap(Box)
  (params (OverlappedComponent :type Primitive%20Component%20Object%20Reference) (OtherActor :type Actor%20Object%20Reference) (OtherComp :type Primitive%20Component%20Object%20Reference) (OtherBodyIndex :type Integer) (bFromSweep :type Boolean) (SweepResult :type Hit%20Result%20Structure%20%28by%20ref%29))
  (Utilities|Casting|CastToL1_Character OtherActor)
  (Game|Player|SetViewTargetwithBlend (Game|GetPlayerController 0) (Variables|Default|GetReferenceRECamera) 0.2 "VTBlend_Linear" 0.0 false)
  (Pawn|SetControlRotation (Game|GetPlayerController 0) (Math|Rotator|MakeRotator 0.0 0.0 (.yaw (Transformation|GetActorRotation (Variables|Default|GetReferenceRECamera)))))
  (Variables|/Game/GameBP/Level1/L1_Character.L1_Character_C|SetIsUseHeadBob (.AsL1%20Character (Utilities|Casting|CastToL1_Character (Game|GetPlayerCharacter 0))) false)
  (Input|SetIgnoreLookInput (Game|GetPlayerController 0) true))

(event EventBeginPlay)

(event Collision|EventActorBeginOverlap
  (params (OtherActor :type Actor%20Object%20Reference)))

(event EventTick
  (params (DeltaSeconds :type Float%20%28single-precision%29)))

(fn ConstructionScript
  (Components|Box|SetBoxExtent (Variables|Default|GetBox) (Variables|Default|GetBoxExtent) true))