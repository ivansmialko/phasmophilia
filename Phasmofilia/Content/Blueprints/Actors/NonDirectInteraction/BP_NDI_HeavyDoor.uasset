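; BP_NDI_HeavyDoor is a non-direct-interaction door actor that slides open or closed each time its Interact event fires.
; A timeline drives a lerp on the Door component's relative X location, playing from start to open and reversing from end to close.
; An in-progress flag ignores interactions while the door moves, and the open state flips when the timeline finishes.
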(event EventBeginPlay
  (|CallParentFunction) ; This node is disabled and will not be called.\nDrag off pins to build functionality.
)

(event Collision|EventActorBeginOverlap
  (params (OtherActor :type Actor%20Object%20Reference))
  (|CallParentFunction OtherActor) ; This node is disabled and will not be called.\nDrag off pins to build functionality.
)

(event EventTick
  (params (DeltaSeconds :type Float%20%28single-precision%29))
  (|CallParentFunction DeltaSeconds) ; This node is disabled and will not be called.\nDrag off pins to build functionality.
)

(event EventInteract
  (bind _door (Variables|Default|GetDoor))
  (bind _relativelocation (Variables|/Script/Engine.SceneComponent|GetRelativeLocation _door))
  (if (not (Variables|Default|GetisDoorOpening))
    (Variables|Default|SetisDoorOpening true)
    (if (Variables|Default|GetisDoorOpen)
      (bind _alpha (Timeline|DoorTL ReverseFromEnd)
        (:Update
          (Transformation|SetRelativeLocation (Variables|Default|GetDoor) (Math|Vector|MakeVector (Math|Float|Lerp 0.0 -1.8e+02 _alpha) (.y _relativelocation) (.z _relativelocation)) false false))
        (:Finished
          (Variables|Default|SetisDoorOpening false)
          (Variables|Default|SetisDoorOpen (not (Variables|Default|GetisDoorOpen)))))
      (else
        (Timeline|DoorTL PlayFromStart)))))

(fn ConstructionScript
  (|CallParentFunction))