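; Base actor for hiding spots that moves the player character between a hiding position and an exit position on interaction.
; Interact starts a looping per-frame timer that interpolates the player at constant speed, disabling collision, movement and inventory when heading into hiding.
; On arrival it fires a finished-moving dispatcher, toggles IsHiding and, depending on the new state, restores those controls or notifies the enemy AI controller of leaving.
; The AI controller is also messaged on entry; EnemyFound is an empty event.
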(event Custom|MoveCharacter
  (bind _playercharacterinstance (Variables|Default|GetPlayerCharacterInstance))
  (Transformation|SetActorTransform _playercharacterinstance (Math|Transform|MakeTransform (Math|Interpolation|VInterptoConstant (Transformation|GetActorLocation _playercharacterinstance) (Transformation|GetWorldLocation (select (Variables|/Game/GameBP/Level1/L1_Character.L1_Character_C|GetIsHiding (Variables|Default|GetPlayerCharacterInstance)) (Variables|Default|GetExitPosititon) (Variables|Default|GetHidingPosition))) (Utilities|Time|GetWorldDeltaSeconds) 1e+03) "0, 0, 0" "1,1,1"))
  (if (Math|Vector|Equal(Vector) (Transformation|GetActorLocation (Variables|Default|GetPlayerCharacterInstance)) (Transformation|GetWorldLocation (select (Variables|/Game/GameBP/Level1/L1_Character.L1_Character_C|GetIsHiding (Variables|Default|GetPlayerCharacterInstance)) (Variables|Default|GetExitPosititon) (Variables|Default|GetHidingPosition))) 0.01)
    (Utilities|Time|ClearandInvalidateTimerbyHandle (stale EventInteract _returnvalue_3))
    (Utilities|Time|ClearandInvalidateTimerbyHandle (stale EventInteract _returnvalue))
    (CallFunction|FinishedMoving)))

(event Custom|FinishedMoving
  (Default|CallFinishedMovingED)
  (bind _output_get (Variables|/Game/GameBP/Level1/L1_Character.L1_Character_C|SetIsHiding (Variables|Default|GetPlayerCharacterInstance) (not (Variables|/Game/GameBP/Level1/L1_Character.L1_Character_C|GetIsHiding (Variables|Default|GetPlayerCharacterInstance)))))
  (if _output_get
    (Collision|SetActorEnableCollision (Variables|Default|GetPlayerCharacterInstance) true)
    (Pawn|Components|CharacterMovement|SetMovementMode (Variables|/Script/Engine.Character|GetCharacterMovement (Variables|Default|GetPlayerCharacterInstance)) "MOVE_Walking" 0)
    (Variables|/Game/GameBP/HG_PlayerController.HG_PlayerController_C|SetIsCanOpenInventory (Variables|Default|GetPlayerControllerInstance) true)
    (else
      (bind _asaic_classic (Utilities|Casting|CastToAIC_ClassicClass "/Game/AI/Classic/AIC_Classic.AIC_Classic_C"))
      (bind _returnvalue (Actor|GetActorOfClass _asaic_classic))
      (Class|BPIPlayerHiding|LeftHidingSpot(Message) _returnvalue))))

(event Custom|EnemyFound)

(event EventBeginPlay
  (Variables|Default|SetPlayerCharacterInstance (.AsL1%20Character (Utilities|Casting|CastToL1_Character (Game|GetPlayerCharacter 0))))
  (bind _ashg_player_controller (Utilities|Casting|CastToHG_PlayerController (Game|GetPlayerController 0)))
  (Variables|Default|SetPlayerControllerInstance _ashg_player_controller))

(event EventInteract
  (params (InteractingCharacter :type Character%20Object%20Reference))
  (if (Variables|/Game/GameBP/Level1/L1_Character.L1_Character_C|GetIsHiding (Variables|Default|GetPlayerCharacterInstance))
    (bind _returnvalue (Utilities|Time|SetTimerbyEvent (delegate Custom|MoveCharacter) (Utilities|Time|GetWorldDeltaSeconds) true))
    (else
      (bind _asaic_classic (Utilities|Casting|CastToAIC_ClassicClass "/Game/AI/Classic/AIC_Classic.AIC_Classic_C"))
      (bind _returnvalue_2 (Actor|GetActorOfClass _asaic_classic))
      (Class|BPIPlayerHiding|DidEnemySee(Message) _returnvalue_2 self)
      (Collision|SetActorEnableCollision (Variables|Default|GetPlayerCharacterInstance) false)
      (Variables|/Game/GameBP/HG_PlayerController.HG_PlayerController_C|SetIsCanOpenInventory (Variables|Default|GetPlayerControllerInstance) false)
      (Pawn|Components|CharacterMovement|DisableMovement (Variables|/Script/Engine.Character|GetCharacterMovement (Variables|Default|GetPlayerCharacterInstance)))
      (bind _returnvalue_3 (Utilities|Time|SetTimerbyEvent (delegate Custom|MoveCharacter) (Utilities|Time|GetWorldDeltaSeconds) true)))))

(fn ConstructionScript)