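; Locker hiding-spot actor that adds an animated door to the interaction logic inherited from its parent hide actor.
; Interact locks out further use, swings the door open with a timeline, then after a brief delay runs the parent Interact.
; The parent's finished-moving dispatcher, bound on BeginPlay, triggers a delayed close timeline, which re-enables interaction when done.
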(event Custom|CloseDoor
  (bind _alpha (Timeline|CloseLockerDoor PlayFromStart)
    (:Update
      (Transformation|SetRelativeRotation (Variables|Default|GetLockerDoor) (Math|Rotator|MakeRotator 0.0 0.0 (Math|Float|Lerp 9e+01 0.0 _alpha)) false false))
    (:Finished
      (Variables|Default|SetCanInteract true))))

(event Custom|FinishedMovingED_Event
  (Utilities|FlowControl|Delay 0.1)
  (CallFunction|CloseDoor))

(event EventBeginPlay
  (|CallParentFunction)
  (EventDispatchers|BindEventtoFinishedMovingED (delegate Custom|FinishedMovingED_Event)))

(event Collision|EventActorBeginOverlap
  (params (OtherActor :type Actor%20Object%20Reference))
  (|CallParentFunction OtherActor) ; This node is disabled and will not be called.\nDrag off pins to build functionality.
)

(event EventTick
  (params (DeltaSeconds :type Float%20%28single-precision%29))
  (|CallParentFunction DeltaSeconds) ; This node is disabled and will not be called.\nDrag off pins to build functionality.
)

(event EventInteract
  (if (Variables|Default|GetCanInteract)
    (Variables|Default|SetCanInteract false)
    (bind _alpha (Timeline|OpenLockerDoor Play)
      (:Update
        (Transformation|SetRelativeRotation (Variables|Default|GetLockerDoor) (Math|Rotator|MakeRotator 0.0 0.0 (Math|Float|Lerp 0.0 9e+01 _alpha)) false false))
      (:Finished
        (Utilities|FlowControl|Delay 0.1)
        (|CallParentFunction)))))

(fn ConstructionScript
  (|CallParentFunction))