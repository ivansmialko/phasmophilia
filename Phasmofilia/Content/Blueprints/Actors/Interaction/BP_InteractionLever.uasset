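; Interactable lever that rotates its key and triggers a linked actor, such as a remote mechanism.
; Interact plays a timeline forward or in reverse depending on IsTurnedUp, lerping LeverKey's roll, with IsTurning blocking re-entry.
; On finish, it messages NonDirectInteractionActor through BPI_NonDirectInteraction.
; The state flip and unlock happen only when that actor is valid and implements the interface, otherwise the lever stays locked.
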(event EventBeginPlay
  (|CallParentFunction) ; This node is disabled and will not be called.\nDrag off pins to build functionality.
)

(event Collision|EventActorBeginOverlap
  (params (OtherActor :type Actor%20Object%20Reference)))

(event EventTick
  (params (DeltaSeconds :type Float%20%28single-precision%29)))

(event EventInteract
  (bind _leverkey (Variables|Default|GetLeverKey))
  (bind _relativerotation (Variables|/Script/Engine.SceneComponent|GetRelativeRotation _leverkey))
  (if (not (Variables|Default|GetisTurning))
    (Variables|Default|SetisTurning true)
    (if (Variables|Default|GetisTurnedUp)
      (bind _alpha (Timeline|LeverTL PlayFromStart)
        (:Update
          (Transformation|SetRelativeRotation _leverkey (Math|Rotator|MakeRotator (Math|Float|Lerp 0.0 105.0 _alpha) (.pitch _relativerotation) (.yaw _relativerotation)) false false))
        (:Finished
          (Utilities|IsValid (Variables|Default|GetNonDirectInteractionActor)
            (:Is%20Valid
              (if (Utilities|DoesObjectImplementInterface (Variables|Default|GetNonDirectInteractionActor) "/Game/Blueprints/Interfaces/BPI_NonDirectInteraction.BPI_NonDirectInteraction_C")
                (Class|BPINonDirectInteraction|Interact(Message) (Variables|Default|GetNonDirectInteractionActor))
                (Variables|Default|SetisTurnedUp (not (Variables|Default|GetisTurnedUp)))
                (Variables|Default|SetisTurning false))))))
      (else
        (Timeline|LeverTL ReverseFromEnd)))))

(fn ConstructionScript
  (|CallParentFunction))