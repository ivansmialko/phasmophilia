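; Interactable door actor that toggles open and closed, always swinging away from the player.
; On opening, the dot product of the player-to-door direction and the door's forward vector picks the yaw sign, and a timeline lerps the mesh rotation.
; Closing reverses that timeline, and each toggle plays a sound through the player controller's audio manager.
; Despite the "Lockable" name, this graph contains no lock check.
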(event EventBeginPlay
  (|CallParentFunction) ; This node is disabled and will not be called.\nDrag off pins to build functionality.
)

(event Collision|EventActorBeginOverlap
  (params (OtherActor :type Actor%20Object%20Reference)))

(event EventInteract
  (params (InteractingCharacter :type Character%20Object%20Reference))
  (bind _self self)
  (if (Variables|Default|GetIsDoorClosed)
    (Variables|Default|SetIsDoorClosed false)
    (CallFunction|PlaySoundDoorOpen)
    (Variables|Default|SetDotProduct (Math|Vector|DotProduct (Math|Vector|Normalize (- (Transformation|GetActorLocation _self) (Transformation|GetActorLocation (Variables|Default|GetPlayerRef)))) (Transformation|GetActorForwardVector _self)))
    (bind _alpha (Timeline|OpenDoorTL Play)
      (:Update
        (Transformation|SetRelativeRotation (Variables|Default|GetStaticMesh1) (Math|Rotator|MakeRotator 0.0 0.0 (Math|Float|Lerp 0.0 (Math|Float|SelectFloat 9e+01 -9e+01 (>= (Variables|Default|GetDotProduct) 0.0)) _alpha)) false false)))
    (else
      (Variables|Default|SetIsDoorClosed true)
      (CallFunction|PlaySoundDoorClosed)
      (Timeline|OpenDoorTL Reverse))))

(fn ConstructionScript
  (|CallParentFunction))

(fn PlaySoundDoorOpen
  (Default|PlayDoorOpen (Variables|/Game/GameBP/HG_PlayerController.HG_PlayerController_C|GetAudioManagerInstance (.AsHG%20Player%20Controller (Utilities|Casting|CastToHG_PlayerController (Game|GetPlayerController 0)))) self))

(fn PlaySoundDoorClosed
  (Default|PlayDoorClose (Variables|/Game/GameBP/HG_PlayerController.HG_PlayerController_C|GetAudioManagerInstance (.AsHG%20Player%20Controller (Utilities|Casting|CastToHG_PlayerController (Game|GetPlayerController 0)))) self))