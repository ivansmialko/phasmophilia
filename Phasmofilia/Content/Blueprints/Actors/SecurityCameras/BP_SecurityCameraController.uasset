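; Interactable security camera console that lets the player view every BP_SecurityCamera in the level.
; On BeginPlay it gathers the cameras; interacting toggles a mode that locks character and look input, hides the main HUD and shows the camera widget.
; While open, SpaceBar cycles the view target with wraparound, and Action or Return exits to the player view.
; Buzz and switch sounds play through the player controller's audio manager.
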(event Custom|EnterCamerasMenu
  (Variables|Default|SetIsOpen true)
  (Input|DisableInput (Game|GetPlayerCharacter 0) (Game|GetPlayerController 0))
  (Input|SetIgnoreLookInput (Game|GetPlayerController 0) true)
  (Widget|SetVisibility (Variables|/Game/GameBP/Level1/L1_Character.L1_Character_C|GetMainHudInstance (.AsL1%20Character (Utilities|Casting|CastToL1_Character (Game|GetPlayerCharacter 0)))) "Hidden")
  (Input|EnableInput (Game|GetPlayerController 0))
  (CallFunction|ViewThroughCamera)
  (UserInterface|Viewport|AddtoViewport (Variables|/Game/GameBP/Level1/L1_Character.L1_Character_C|GetCameraWidgetInstance (.AsL1%20Character (Utilities|Casting|CastToL1_Character (Game|GetPlayerCharacter 0)))) 0)
  (CallFunction|PlaySoundCameraBuzz))

(event Custom|LeaveCamerasMenu
  (Variables|Default|SetIsOpen false)
  (Input|EnableInput (Game|GetPlayerCharacter 0) (Game|GetPlayerController 0))
  (Input|ResetIgnoreLookInput (Game|GetPlayerController 0))
  (Widget|SetVisibility (Variables|/Game/GameBP/Level1/L1_Character.L1_Character_C|GetMainHudInstance (.AsL1%20Character (Utilities|Casting|CastToL1_Character (Game|GetPlayerCharacter 0)))) "SelfHitTestInvisible")
  (Input|DisableInput (Game|GetPlayerController 0))
  (Game|Player|SetViewTargetwithBlend (Game|GetPlayerController 0) (Game|GetPlayerCharacter 0) 0.0 "VTBlend_Linear" 0.0 false)
  (Widget|RemovefromParent (Variables|/Game/GameBP/Level1/L1_Character.L1_Character_C|GetCameraWidgetInstance (.AsL1%20Character (Utilities|Casting|CastToL1_Character (Game|GetPlayerCharacter 0)))))
  (CallFunction|StopSoundCameraBuzz))

(event EventBeginPlay
  (bind _outactors (Actor|GetAllActorsOfClass "/Game/Blueprints/Actors/SecurityCameras/BP_SecurityCamera.BP_SecurityCamera_C"))
  (Variables|Default|SetSecurityCamerasList _outactors))

(event EventInteract
  (if (Variables|Default|GetIsOpen)
    (CallFunction|LeaveCamerasMenu)
    (else
      (CallFunction|EnterCamerasMenu))))

(event Input|ActionEvents|InputActionAction
  (params (Key :type Key%20Structure :default "None"))
  (:Pressed
    (CallFunction|LeaveCamerasMenu)))

(event Input|ActionEvents|InputActionReturn
  (params (Key :type Key%20Structure :default "None"))
  (:Pressed
    (CallFunction|LeaveCamerasMenu)))

(event Input|KeyboardEvents|SpaceBar
  (params (Key :type Key%20Structure :default "None"))
  (:Pressed
    (Variables|Default|SetCurrentCameraIndex (select (> (+ (Variables|Default|GetCurrentCameraIndex) 1) (- (Utilities|Array|Length (Variables|Default|GetSecurityCamerasList)) 1)) 0 (+ (Variables|Default|GetCurrentCameraIndex) 1)))
    (CallFunction|ViewThroughCamera)
    (CallFunction|PlaySoundCameraSwitch)))

(fn ConstructionScript)

(fn ViewThroughCamera
  (Game|Player|SetViewTargetwithBlend (Game|GetPlayerController 0) (Utilities|Array|Get(acopy) (Variables|Default|GetSecurityCamerasList) (Variables|Default|GetCurrentCameraIndex)) 0.0 "VTBlend_Linear" 0.0 false)
  (return))

(fn PlaySoundCameraSwitch
  (Default|PlayCameraSwitch (Variables|/Game/GameBP/HG_PlayerController.HG_PlayerController_C|GetAudioManagerInstance (.AsHG%20Player%20Controller (Utilities|Casting|CastToHG_PlayerController (Game|GetPlayerController 0))))))

(fn PlaySoundCameraBuzz
  (Default|PlayCameraBuzz (Variables|/Game/GameBP/HG_PlayerController.HG_PlayerController_C|GetAudioManagerInstance (.AsHG%20Player%20Controller (Utilities|Casting|CastToHG_PlayerController (Game|GetPlayerController 0))))))

(fn StopSoundCameraBuzz
  (Default|StopCameraBuzz (Variables|/Game/GameBP/HG_PlayerController.HG_PlayerController_C|GetAudioManagerInstance (.AsHG%20Player%20Controller (Utilities|Casting|CastToHG_PlayerController (Game|GetPlayerController 0))))))