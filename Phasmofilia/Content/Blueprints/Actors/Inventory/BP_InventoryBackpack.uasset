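; Backpack pickup actor that adds slots to the player's inventory component and destroys itself when the Action input is pressed.
; Sphere overlap with L1_Character shows a prompt widget and activates per-tick updates.
; Tick keeps the prompt above the mesh, line-traces to the player's camera to hide it when blocked, and otherwise turns it toward the camera.
; Actor input is enabled only when unobstructed and within pickup distance, which also toggles the prompt's state.
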(event OnComponentBeginOverlap(Sphere)
  (params (OverlappedComponent :type Primitive%20Component%20Object%20Reference) (OtherActor :type Actor%20Object%20Reference) (OtherComp :type Primitive%20Component%20Object%20Reference) (OtherBodyIndex :type Integer) (bFromSweep :type Boolean) (SweepResult :type Hit%20Result%20Structure%20%28by%20ref%29))
  (bind _asl1_character (Utilities|Casting|CastToL1_Character OtherActor))
  (Variables|Default|SetPlayerCharacterInstance _asl1_character)
  (Rendering|SetVisibility (Variables|Default|GetPrompt) true false)
  (Variables|Default|SetUpdate%20Actor true))

(event OnComponentEndOverlap(Sphere)
  (params (OverlappedComponent :type Primitive%20Component%20Object%20Reference) (OtherActor :type Actor%20Object%20Reference) (OtherComp :type Primitive%20Component%20Object%20Reference) (OtherBodyIndex :type Integer))
  (Utilities|Casting|CastToL1_Character OtherActor)
  (Rendering|SetVisibility (Variables|Default|GetPrompt) false false)
  (Variables|Default|SetUpdate%20Actor false)
  (Input|DisableInput (Game|GetPlayerController 0)))

(event EventBeginPlay)

(event Collision|EventActorBeginOverlap
  (params (OtherActor :type Actor%20Object%20Reference)))

(event EventTick
  (params (DeltaSeconds :type Float%20%28single-precision%29))
  (bind _backpack (Variables|Default|GetBackPack))
  (bind _returnvalue (Transformation|GetWorldLocation _backpack))
  (Transformation|SetWorldLocation (Variables|Default|GetPrompt) (Math|Vector|MakeVector (.x _returnvalue) (.y _returnvalue) (+ (.z _returnvalue) (Variables|Default|GetWidget%20Distance%20Above%20Mesh))) false false)
  (if (Variables|Default|GetUpdate%20Actor)
    (bind (_outhit _returnvalue_2) (Collision|LineTraceByChannel (Transformation|GetActorLocation) (Transformation|GetWorldLocation (Variables|/Game/GameBP/Level1/L1_Character.L1_Character_C|GetCamera (Variables|Default|GetPlayerCharacterInstance))) "TraceTypeQuery1" false 0 "None" true "(R=1.000000,G=0.000000,B=0.000000,A=1.000000)" "(R=0.000000,G=1.000000,B=0.000000,A=1.000000)" 1.0))
    (if _returnvalue_2
      (Rendering|SetVisibility (Variables|Default|GetPrompt) false false)
      (Input|DisableInput (Game|GetPlayerController 0))
      (else
        (Rendering|SetVisibility (Variables|Default|GetPrompt) true false)
        (Transformation|SetWorldRotation (Variables|Default|GetPrompt) (Math|Rotator|FindLookatRotation (Transformation|GetWorldLocation (Variables|Default|GetPrompt)) (Transformation|GetWorldLocation (Variables|/Game/GameBP/Level1/L1_Character.L1_Character_C|GetCamera (Variables|Default|GetPlayerCharacterInstance)))) false false)
        (bind _asw_pick_up_prompt (Utilities|Casting|CastToW_PickUpPrompt (UserInterface|GetUserWidgetObject (Variables|Default|GetPrompt))))
        (Default|TogglePrompt _asw_pick_up_prompt (<= (Math|Vector|VectorLength (- (.TraceStart (Collision|BreakHitResult _outhit)) (.TraceEnd (Collision|BreakHitResult _outhit)))) (Variables|Default|GetPick%20Up%20Distance)))
        (if (<= (Math|Vector|VectorLength (- (.TraceStart (Collision|BreakHitResult _outhit)) (.TraceEnd (Collision|BreakHitResult _outhit)))) (Variables|Default|GetPick%20Up%20Distance))
          (Input|EnableInput (Game|GetPlayerController 0))
          (else
            (Input|DisableInput (Game|GetPlayerController 0))))))))

(event Input|ActionEvents|InputActionAction
  (params (Key :type Key%20Structure :default "None"))
  (:Pressed
    (Default|AddMoreSlots (Variables|/Game/GameBP/Level1/L1_Character.L1_Character_C|GetBPC_Inventory (Variables|Default|GetPlayerCharacterInstance)) (Variables|Default|GetAmountOfSlots))
    (Actor|DestroyActor)))

(fn ConstructionScript)