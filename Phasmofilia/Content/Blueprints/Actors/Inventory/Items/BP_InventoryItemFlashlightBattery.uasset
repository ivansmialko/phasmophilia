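; Inventory item Blueprint for a flashlight battery that recharges the player's flashlight when used.
; UseItem adds BatteryAmount to the player's flashlight component only while its battery is below maximum, otherwise it flags the use as failed.
; A successful use also completes the "UseBattery" objective through the GameState, without immediately setting the next objective.
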(event EventBeginPlay
  (|CallParentFunction) ; This node is disabled and will not be called.\nDrag off pins to build functionality.
)

(event Collision|EventActorBeginOverlap
  (params (OtherActor :type Actor%20Object%20Reference))
  (|CallParentFunction OtherActor) ; This node is disabled and will not be called.\nDrag off pins to build functionality.
)

(event EventTick
  (params (DeltaSeconds :type Float%20%28single-precision%29))
  (|CallParentFunction DeltaSeconds) ; This node is disabled and will not be called.\nDrag off pins to build functionality.
)

(event EventUseItem
  (bind _playercharacterinstance (Variables|Default|GetPlayerCharacterInstance))
  (bind _bpc_flashlight (Variables|/Game/GameBP/Level1/L1_Character.L1_Character_C|GetBPC_Flashlight _playercharacterinstance))
  (if (< (Variables|/Game/Blueprints/BlueprintComponents/BPC_Flashlight.BPC_Flashlight_C|GetCurrentBateryLevel _bpc_flashlight) (Variables|/Game/Blueprints/BlueprintComponents/BPC_Flashlight.BPC_Flashlight_C|GetMaxBatteryLevel _bpc_flashlight))
    (Default|AddBatteryLife (Variables|/Game/GameBP/Level1/L1_Character.L1_Character_C|GetBPC_Flashlight (Variables|Default|GetPlayerCharacterInstance)) (Variables|Default|GetBatteryAmount))
    (Variables|Default|SetItemUseSuccessfull true)
    (Class|BPIObjectiveCall|CompleteObjectiveCall(Message) (Game|GetGameState) "UseBattery" false)
    (else
      (Variables|Default|SetItemUseSuccessfull false))))

(fn ConstructionScript
  (|CallParentFunction))