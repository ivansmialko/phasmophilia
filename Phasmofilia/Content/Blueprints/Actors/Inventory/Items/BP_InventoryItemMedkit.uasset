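; BP_InventoryItemMedkit is an inventory item that heals the player character when used.
; UseItem compares current and max health on the player's BPCHealthComponent and adds HealingAmount only when health is below max.
; Both branches set ItemUseSuccessfull to true, so the use reports success even at full health when no healing occurs.
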(event EventBeginPlay
  (|CallParentFunction) ; This node is disabled and will not be called.\nDrag off pins to build functionality.
)

(event Collision|EventActorBeginOverlap
  (params (OtherActor :type Actor%20Object%20Reference))
  (|CallParentFunction OtherActor) ; This node is disabled and will not be called.\nDrag off pins to build functionality.
)

(event EventTick
  (params (DeltaSeconds :type Float%20%28single-precision%29))
  (|CallParentFunction DeltaSeconds) ; This node is disabled and will not be called.\nDrag off pins to build functionality.
)

(event EventUseItem
  (bind _playercharacterinstance (Variables|Default|GetPlayerCharacterInstance))
  (bind _bpc_healthcomponent (Variables|/Game/GameBP/Level1/L1_Character.L1_Character_C|GetBPC_HealthComponent _playercharacterinstance))
  (if (< (Variables|/Game/Blueprints/BlueprintComponents/BPC_HealthComponent.BPC_HealthComponent_C|GetCurrentHealth _bpc_healthcomponent) (Variables|/Game/Blueprints/BlueprintComponents/BPC_HealthComponent.BPC_HealthComponent_C|GetMaxHealth _bpc_healthcomponent))
    (Default|AddHealth (Variables|/Game/GameBP/Level1/L1_Character.L1_Character_C|GetBPC_HealthComponent (Variables|Default|GetPlayerCharacterInstance)) (Variables|Default|GetHealingAmount))
    (Variables|Default|SetItemUseSuccessfull true)
    (else
      (Variables|Default|SetItemUseSuccessfull true))))

(fn ConstructionScript
  (|CallParentFunction))